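; BP_GestureCollider is a collider that applies a gesture pose to a VR character's hand while it overlaps.
; On begin overlap it identifies the hand from the grip motion controller and calls SetPose without override.
; If that fails, it binds to the character's drop event to force the pose later.
; End overlap clears the pose and unbinds; a helper resolving character, controller and grasping hand sits unused by the event graph.
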(event `self.ReceiveBeginPlay`
  (`|ExecutionSequence`
    (:`then_0`
      (add `self.OnComponentBeginOverlap` (delegate `ComponentOverlap_`)))
    (:`then_1`
      (add `self.OnComponentEndOverlap` (delegate `ComponentOverlapEnd`)))))

(event `ComponentOverlap_` :!signature `self.OnComponentBeginOverlap`
  (params (OverlappedComponent :type "PrimitiveComponent Object Reference") (OtherActor :type "Actor Object Reference") (OtherComp :type "PrimitiveComponent Object Reference") (OtherBodyIndex :type Integer) (bFromSweep :type Boolean) (SweepResult :type "HitResult Structure (by ref)"))
  (bind _asbp_vrcharacter_dvree (cast `/DVREE_GestureCollider/Blueprints/BP_VRCharacterDVREE` OtherActor))
  (bind _asgrip_motion_controller_component (cast `GripMotionControllerComponent` (`self.GetAttachParent` OtherComp)))
  (bind _succeeded (`/DVREE_GestureCollider/Blueprints/BP_VRCharacterDVREE.SetPose` _asbp_vrcharacter_dvree (`self.gesturePose`) (`GripMotionControllerComponent.GetHandType` _asgrip_motion_controller_component) false))
  (if (not _succeeded)
    (add `/DVREE_GestureCollider/Blueprints/BP_VRCharacterDVREE.OnDrop` _asbp_vrcharacter_dvree (delegate `manualOnOverlapCall`))))

(event `manualOnOverlapCall`
  (params (DroppingVRCharacter :type "/DVREE_GestureCollider/Blueprints/BP_VRCharacterDVREE Object Reference") (DroppingController :type "EControllerHand Enum" :default "Left"))
  (`/Engine/EditorBlueprintResources/StandardMacros.IsValid` DroppingVRCharacter
    (:`Is Valid`
      (`/DVREE_GestureCollider/Blueprints/BP_VRCharacterDVREE.SetPose` DroppingVRCharacter (`self.gesturePose`) DroppingController true)
      (remove `/DVREE_GestureCollider/Blueprints/BP_VRCharacterDVREE.OnDrop` DroppingVRCharacter (delegate `manualOnOverlapCall`)))))

(event `ComponentOverlapEnd` :!signature `self.OnComponentEndOverlap`
  (params (OverlappedComponent :type "PrimitiveComponent Object Reference") (OtherActor :type "Actor Object Reference") (OtherComp :type "PrimitiveComponent Object Reference") (OtherBodyIndex :type Integer))
  (bind _asbp_vrcharacter_dvree (cast `/DVREE_GestureCollider/Blueprints/BP_VRCharacterDVREE` OtherActor))
  (bind _asgrip_motion_controller_component (cast `GripMotionControllerComponent` (`self.GetAttachParent` OtherComp)))
  (bind _succeeded (`/DVREE_GestureCollider/Blueprints/BP_VRCharacterDVREE.SetPose` _asbp_vrcharacter_dvree null (`GripMotionControllerComponent.GetHandType` _asgrip_motion_controller_component) true))
  (if _succeeded
    _
    (else
      _))
  (bind _asbp_vrcharacter_dvree_2 (cast `/DVREE_GestureCollider/Blueprints/BP_VRCharacterDVREE` OtherActor))
  (remove `/DVREE_GestureCollider/Blueprints/BP_VRCharacterDVREE.OnDrop` _asbp_vrcharacter_dvree_2 (delegate `manualOnOverlapCall`)))

(fn `Get Parameters`
  (params (OverlappedActor :type "Object Object Reference") (OverlappedComponent :type "PrimitiveComponent Object Reference"))
  (returns (VRCharacter :type "VRCharacter Object Reference") (GrabSphere :type "PrimitiveComponent Object Reference") (MotionController :type "MotionControllerComponent Object Reference") (GraspingHand :type "/Game/VRE/Core/GraspingHands/GraspingHandManny Object Reference") (Succeeded :type Boolean))
  (bind _returnvalue (`self.GetAttachParent` OverlappedComponent))
  (if (`KismetMathLibrary.ClassIsChildOf` (`GameplayStatics.GetObjectClass` OverlappedActor) "/Game/VRE/Core/Character/BP_VRCharacter.BP_VRCharacter_C")
    (bind _asbp_vrcharacter (cast `/Game/VRE/Core/Character/BP_VRCharacter` OverlappedActor)
      (:`then`
        (`/Engine/EditorBlueprintResources/StandardMacros.IsValid` _returnvalue
          (:`Is Valid`
            (bind _asmotion_controller_component (cast `MotionControllerComponent` _returnvalue)
              (:`then`
                (switch `name` (`MotionControllerComponent.MotionSource` _asmotion_controller_component)
                  (:`left`
                    (return _asbp_vrcharacter OverlappedComponent _asmotion_controller_component (`/Game/VRE/Core/Character/BP_VRCharacter.GraspingHandLeft` _asbp_vrcharacter) true))
                  (:`right`
                    (return _asbp_vrcharacter OverlappedComponent _asmotion_controller_component (`/Game/VRE/Core/Character/BP_VRCharacter.GraspingHandRight` _asbp_vrcharacter) true))))
              (:`CastFailed`
                _)))
          (:`Is Not Valid`
            _)))
      (:`CastFailed`
        _)))
  (return null null null null false))